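; BP_Fragment is a collectible pickup that adds to the first-person character's Zakladka counter.
; Entering its Box enables player input on the actor, caches the character and shows a text prompt for a few seconds; leaving disables input.
; TakeZakladaka increments and prints the count, destroys the fragment and calls Frag on the character's Aim2.
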(event OnComponentBeginOverlap(Box)
  (params (OverlappedComponent :type Primitive%20Component%20Object%20Reference) (OtherActor :type Actor%20Object%20Reference) (OtherComp :type Primitive%20Component%20Object%20Reference) (OtherBodyIndex :type Integer) (bFromSweep :type Boolean) (SweepResult :type Hit%20Result%20Structure%20%28by%20ref%29))
  (bind _textrender (Variables|Default|GetTextRender))
  (Input|EnableInput (Game|GetPlayerController 0))
  (bind _asbp_first_person_character (Utilities|Casting|CastToBP_FirstPersonCharacter OtherActor))
  (Rendering|SetVisibility _textrender true false)
  (Utilities|FlowControl|Delay 3.0)
  (Rendering|SetVisibility _textrender false false))

(event OnComponentEndOverlap(Box)
  (params (OverlappedComponent :type Primitive%20Component%20Object%20Reference) (OtherActor :type Actor%20Object%20Reference) (OtherComp :type Primitive%20Component%20Object%20Reference) (OtherBodyIndex :type Integer))
  (Input|DisableInput (Game|GetPlayerController 0)))

(event Custom|TakeZakladaka
  (bind _result (Math|Integer|IncrementInt (Variables|/Game/FirstPerson/Blueprints/BP_FirstPersonCharacter.BP_FirstPersonCharacter_C|Getzakladka (stale OnComponentBeginOverlap(Box) _asbp_first_person_character)))
    (:%20%20
      (bind _output_get (Variables|/Game/FirstPerson/Blueprints/BP_FirstPersonCharacter.BP_FirstPersonCharacter_C|Setzakladka (stale OnComponentBeginOverlap(Box) _asbp_first_person_character) _result))
      (Development|PrintString (Utilities|String|ToString(Integer) _output_get))
      (Actor|DestroyActor)
      (Default|Frag (Variables|/Game/FirstPerson/Blueprints/BP_FirstPersonCharacter.BP_FirstPersonCharacter_C|GetAim2 (stale OnComponentBeginOverlap(Box) _asbp_first_person_character))))))

(event Input|KeyboardEvents|E
  (params (Key :type Key%20Structure :default "None")))

(fn ConstructionScript)