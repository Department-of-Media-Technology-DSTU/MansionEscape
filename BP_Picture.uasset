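; BP_Picture is an interactable picture actor that briefly shows an on-screen text widget.
; Box overlap enables player input and shows a TextRender prompt, and end overlap reverses both without checking which actor overlapped.
; The Picture event adds a W_PictureText widget to the viewport and removes it after a short delay, using a DoOnce that resets afterward to block repeat triggers meanwhile.
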(event OnComponentBeginOverlap(Box)
  (params (OverlappedComponent :type Primitive%20Component%20Object%20Reference) (OtherActor :type Actor%20Object%20Reference) (OtherComp :type Primitive%20Component%20Object%20Reference) (OtherBodyIndex :type Integer) (bFromSweep :type Boolean) (SweepResult :type Hit%20Result%20Structure%20%28by%20ref%29))
  (Input|EnableInput (Game|GetPlayerController 0))
  (Rendering|SetVisibility (Variables|Default|GetTextRender) true false))

(event OnComponentEndOverlap(Box)
  (params (OverlappedComponent :type Primitive%20Component%20Object%20Reference) (OtherActor :type Actor%20Object%20Reference) (OtherComp :type Primitive%20Component%20Object%20Reference) (OtherBodyIndex :type Integer))
  (Input|DisableInput (Game|GetPlayerController 0))
  (Rendering|SetVisibility (Variables|Default|GetTextRender) false false))

(event Custom|Picture
  (params (NewParam :type Actor%20Object%20Reference))
  (Utilities|FlowControl|DoOnce false :!label _label
    (:Completed
      (bind _returnvalue (UserInterface|CreateWidget "/Game/MyGame/Widgets/W_PictureText.W_PictureText_C"))
      (UserInterface|Viewport|AddtoViewport _returnvalue 0)
      (Utilities|FlowControl|Delay 2.0)
      (Widget|RemovefromParent _returnvalue)
      (goto _label Reset))))

(fn ConstructionScript)