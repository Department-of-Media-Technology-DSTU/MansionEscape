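; Keypad-locked door that plays a one-time applause gag when opened.
; Interaction opens a UI_KeyPad widget in UI-only input until CheckCode matches ValidCode, then later interactions toggle the door.
; A Timeline drives the Arrow's yaw forward or in reverse, with a DoOnce on its update spawning a temporary BP_Clapping actor and sounds at fixed coordinates.
; Box overlap briefly shows an interact prompt.
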(event OnComponentBeginOverlap(Box)
  (params (OverlappedComponent :type Primitive%20Component%20Object%20Reference) (OtherActor :type Actor%20Object%20Reference) (OtherComp :type Primitive%20Component%20Object%20Reference) (OtherBodyIndex :type Integer) (bFromSweep :type Boolean) (SweepResult :type Hit%20Result%20Structure%20%28by%20ref%29))
  (bind _f_to_interract (Variables|Default|GetF%20to%20interract))
  (Rendering|SetVisibility _f_to_interract true false)
  (Utilities|FlowControl|Delay 3.0)
  (Rendering|SetVisibility _f_to_interract false false))

(event OnComponentEndOverlap(Box)
  (params (OverlappedComponent :type Primitive%20Component%20Object%20Reference) (OtherActor :type Actor%20Object%20Reference) (OtherComp :type Primitive%20Component%20Object%20Reference) (OtherBodyIndex :type Integer))
  (Rendering|SetVisibility (Variables|Default|GetF%20to%20interract) false false))

(event Custom|CheckCode
  (params (CurrentCode :type String))
  (bind _returnvalue (Game|GetPlayerController 0))
  (if (Utilities|Enum|Equal(Enum) CurrentCode (Variables|Default|GetValidCode))
    (Audio|PlaySound2D "/Game/MyGame/Sounds/Safe/Acsess_Granted.Acsess_Granted" 1.0 1.0 0.0 0 0)
    (Variables|Default|SetValidCodeEntered true)
    (Widget|RemovefromParent (Variables|Default|GetWidget))
    (Variables|/Script/Engine.PlayerController|SetbShowMouseCursor _returnvalue false)
    (Input|SetInputModeGameOnly _returnvalue false)
    (else
      (Audio|PlaySound2D "/Game/MyGame/Sounds/Safe/Acsess_denied.Acsess_denied" 1.0 1.0 0.0 0 0)
      (Variables|Default|SetValidCodeEntered false))))

(event Custom|OpenCloseDoor
  (bind _output_get (Variables|Default|Setclosed (not (Variables|Default|Getclosed))))
  (if _output_get
    (Audio|PlaySound2D "/Game/MyGame/Sounds/Safe/Safe_open.Safe_open" 0.1 1.0 0.0 0 0)
    (bind _newtrack_0 (Timeline|Timeline Play)
      (:Update
        (Transformation|SetRelativeRotation (Variables|Default|GetArrow) (Math|Rotator|MakeRotator 0.0 0.0 _newtrack_0) false false)
        (Variables|Default|Setclosed (> _newtrack_0 89.0))
        (Utilities|FlowControl|DoOnce false
          (:Completed
            (bind _returnvalue (Game|SpawnActorfromClass "/Game/MyGame/BluePrints/Animation/BP_Clapping.BP_Clapping_C" (Math|Transform|MakeTransform "535.410000,516.810000,139.470000" "0, 0, 0" "1.000000,1.000000,1.000000") "Undefined" "MultiplyWithRoot" 0 0))
            (Audio|SpawnSoundatLocation "/Game/MyGame/Sounds/Clap/Clap.Clap" "566.430000,531.010000,198.390000" "0, 0, 0" 1.0 1.0 0.0 0 0)
            (Audio|SpawnSoundatLocation "/Game/MyGame/Sounds/Hohot/Hohot.Hohot" "566.430000,531.010000,198.390000" "0, 0, 0" 1.0 1.0 0.0 0 0)
            (Utilities|FlowControl|Delay 5.0)
            (Actor|DestroyActor _returnvalue)))))
    (else
      (Audio|PlaySound2D "/Game/MyGame/Sounds/Safe/Safe_open.Safe_open" 0.1 1.0 0.0 0 0)
      (Timeline|Timeline Reverse))))

(fn ConstructionScript)

(fn Interaction
  (bind _returnvalue (Game|GetPlayerController 0))
  (if (Variables|Default|GetValidCodeEntered)
    (CallFunction|OpenCloseDoor)
    (else
      (Audio|PlaySound2D "/Game/MyGame/Sounds/Personazh/Mne_nuzhen_pass.Mne_nuzhen_pass" 0.75 1.0 0.0 0 0)
      (bind _returnvalue_2 (UserInterface|CreateWidget "/Game/MyGame/BluePrints/Seif/UI_KeyPad.UI_KeyPad_C"))
      (Variables|Default|SetWidget _returnvalue_2)
      (UserInterface|Viewport|AddtoViewport _returnvalue_2 0)
      (Variables|/Script/Engine.PlayerController|SetbShowMouseCursor _returnvalue true)
      (Input|SetInputModeUIOnly _returnvalue _returnvalue_2 "DoNotLock" false)
      (return true))))