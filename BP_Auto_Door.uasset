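; Sliding door Blueprint that toggles open and shut through an AutoDoor event, with a box trigger marking the interaction zone.
; Entering the box enables player input and shows a text render for a few seconds; leaving disables input and hides it.
; AutoDoor flips a Closed flag, plays a 2D slide sound, and plays or reverses a Timeline.
; The Timeline drives an Arrow component's relative X location and rewrites Closed from its track value.
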(event OnComponentBeginOverlap(Box)
  (params (OverlappedComponent :type Primitive%20Component%20Object%20Reference) (OtherActor :type Actor%20Object%20Reference) (OtherComp :type Primitive%20Component%20Object%20Reference) (OtherBodyIndex :type Integer) (bFromSweep :type Boolean) (SweepResult :type Hit%20Result%20Structure%20%28by%20ref%29))
  (bind _textrender (Variables|Default|GetTextRender))
  (Input|EnableInput (Game|GetPlayerController 0))
  (Rendering|SetVisibility _textrender true false)
  (Utilities|FlowControl|Delay 3.0)
  (Rendering|SetVisibility _textrender false false))

(event OnComponentEndOverlap(Box)
  (params (OverlappedComponent :type Primitive%20Component%20Object%20Reference) (OtherActor :type Actor%20Object%20Reference) (OtherComp :type Primitive%20Component%20Object%20Reference) (OtherBodyIndex :type Integer))
  (Input|DisableInput (Game|GetPlayerController 0))
  (Rendering|SetVisibility (Variables|Default|GetTextRender) false false))

(event Custom|AutoDoor
  (bind _output_get (Variables|Default|Setclosed (not (Variables|Default|Getclosed))))
  (if _output_get
    (Audio|PlaySound2D "/Game/MyGame/Sounds/Doors/SlideDver.SlideDver" 0.1 1.0 0.0 0 0)
    (bind _newtrack_0 (Timeline|Timeline Play)
      (:Update
        (Transformation|SetRelativeLocation (Variables|Default|GetArrow) (Math|Vector|MakeVector _newtrack_0 0.0 0.0) false false)
        (Variables|Default|Setclosed (> _newtrack_0 99.0))))
    (else
      (Audio|PlaySound2D "/Game/MyGame/Sounds/Doors/SlideDver.SlideDver" 0.1 1.0 0.0 0 0)
      (Timeline|Timeline Reverse))))

(event EventBeginPlay)

(event Collision|EventActorBeginOverlap
  (params (OtherActor :type Actor%20Object%20Reference)))

(event EventTick
  (params (DeltaSeconds :type Float%20%28single-precision%29)))

(fn ConstructionScript)