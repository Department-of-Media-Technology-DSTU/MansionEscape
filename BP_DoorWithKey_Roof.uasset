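; Roof door actor that the first-person character can open only while holding the roof key (Keyroof).
; Box overlap checks the key, then either enables input and shows a timed prompt or shows a timed error text; leaving disables input and hides both.
; OpenDoor toggles Closed, plays a sound and plays or reverses a Timeline that yaws the Arrow component, which also rewrites Closed from the angle.
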(event OnComponentBeginOverlap(Box)
  (params (OverlappedComponent :type Primitive%20Component%20Object%20Reference) (OtherActor :type Actor%20Object%20Reference) (OtherComp :type Primitive%20Component%20Object%20Reference) (OtherBodyIndex :type Integer) (bFromSweep :type Boolean) (SweepResult :type Hit%20Result%20Structure%20%28by%20ref%29))
  (bind _textrender (Variables|Default|GetTextRender))
  (bind _error (Variables|Default|GetError))
  (bind _asbp_first_person_character (Utilities|Casting|CastToBP_FirstPersonCharacter OtherActor))
  (if (Variables|/Game/FirstPerson/Blueprints/BP_FirstPersonCharacter.BP_FirstPersonCharacter_C|Getkeyroof _asbp_first_person_character)
    (Input|EnableInput (Game|GetPlayerController 0))
    (Rendering|SetVisibility _textrender true false)
    (Utilities|FlowControl|Delay 3.0)
    (Rendering|SetVisibility _textrender false false)
    (else
      (Rendering|SetVisibility _error true false)
      (Utilities|FlowControl|Delay 3.0)
      (Rendering|SetVisibility _error false false))))

(event OnComponentEndOverlap(Box)
  (params (OverlappedComponent :type Primitive%20Component%20Object%20Reference) (OtherActor :type Actor%20Object%20Reference) (OtherComp :type Primitive%20Component%20Object%20Reference) (OtherBodyIndex :type Integer))
  (Input|DisableInput (Game|GetPlayerController 0))
  (Rendering|SetVisibility (Variables|Default|GetTextRender) false false))

(event Input|ActionEvents|InputActionOpenDoor
  (params (Key :type Key%20Structure :default "None"))
  (:Pressed
    (bind _output_get (Variables|Default|Setclosed (not (Variables|Default|Getclosed))))
    (if _output_get
      (Audio|PlaySound2D "/Game/MyGame/Sounds/Doors/DoorOpen.DoorOpen" 0.1 1.0 0.0 0 0)
      (bind _newtrack_0 (Timeline|Timeline Play)
        (:Update
          (Transformation|SetRelativeRotation (Variables|Default|GetArrow) (Math|Rotator|MakeRotator 0.0 0.0 _newtrack_0) false false)
          (Variables|Default|Setclosed (> _newtrack_0 89.0))))
      (else
        (Audio|PlaySound2D "/Game/MyGame/Sounds/Doors/DoorOpen.DoorOpen" 0.1 1.0 0.0 0 0)
        (Timeline|Timeline Reverse)))))

(fn ConstructionScript)